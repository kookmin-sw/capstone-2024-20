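; BP_BrokenRock is a destructible rock terrain actor that shatters when hit.
; On hit, it destroys the Rock4 component, enables physics on a Geometry Collection and fires a RadialForce impulse to scatter the fragments.
; Timers then switch the debris to a custom collision channel after a few seconds and later destroy the whole actor.
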(event `self.Rock4.OnComponentHit`
  (params (HitComponent :type "PrimitiveComponent Object Reference") (OtherActor :type "Actor Object Reference") (OtherComp :type "PrimitiveComponent Object Reference") (NormalImpulse :type "Vector Structure") (Hit :type "HitResult Structure (by ref)"))
  (`ActorComponent.K2_DestroyComponent` (`self.Rock4`))
  (`PrimitiveComponent.SetSimulatePhysics` (`self.GeometryCollection`) true)
  (`RadialForceComponent.FireImpulse` (`self.RadialForce`))
  (`KismetSystemLibrary.K2_SetTimer` null "TimerDown" 7.0)
  (`KismetSystemLibrary.K2_SetTimer` null "TimerDestroy" 14.0))

(fn `TimerDestroy`
  (`self.K2_DestroyActor`))

(fn `TimerDown`
  (`PrimitiveComponent.SetCollisionObjectType` (`self.GeometryCollection`) "ECC_GameTraceChannel1"))

(fn `UserConstructionScript`)